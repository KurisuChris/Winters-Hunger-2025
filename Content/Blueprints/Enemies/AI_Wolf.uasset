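; AI_Wolf is an enemy wolf that roams, chases the player and attacks.
; It repeatedly moves to random nearby navigable points until PawnSensing sees any pawn, then barks and moves to player 0.
; On arrival, it applies damage via a forward sphere trace and resumes roaming; both branch conditions are hardwired true, leaving the Player tag check unused.
; StartShot kills it instantly with a death sound.
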(event `self.ReceiveBeginPlay`
  (`self.RandomRoam`))

(event `RandomRoam`
  (bind _randomlocation (`NavigationSystemV1.K2_GetRandomLocationInNavigableRadius` (`self.K2_GetActorLocation`) 1000.0 null null))
  (`|AIMoveTo` self _randomlocation null
    (:`OnSuccess`
      (`KismetSystemLibrary.Delay` 0.2)
      (`self.RandomRoam`))))

(event `self.PawnSensing.OnSeePawn`
  (params (Pawn :type "Pawn Object Reference"))
  (bind _returnvalue (`self.K2_GetActorLocation`))
  (if true
    (`GameplayStatics.SpawnSoundAttached` "/Game/Audio/SFX/Wolf/Barks/SC_Wolf_Barks.SC_Wolf_Barks" (`self.Audio`) "None" (0.0 0.0 0.0) (struct) "KeepRelativeOffset" false 1.0 1.0 0.0 null null)
    (`|AIMoveTo` self (0.0 0.0 0.0) (`GameplayStatics.GetPlayerCharacter` 0) 200.0
      (:`OnSuccess`
        (`KismetSystemLibrary.PrintString` "Attack")
        (bind _outhit (`KismetSystemLibrary.SphereTraceSingleForObjects` _returnvalue (+ _returnvalue (* (`KismetMathLibrary.GetForwardVector` (`self.K2_GetActorRotation`)) 500.0)) 350.0 (`|MakeArray` "ObjectTypeQuery3" :!type "EObjectTypeQuery Enum")))
        (if true
          (`GameplayStatics.SpawnSoundAttached` "/Game/Audio/SFX/Wolf/Attack/SC_Attack.SC_Attack" (`self.Audio`) "None" (0.0 0.0 0.0) (struct) "KeepRelativeOffset" false 1.0 1.0 0.0 null null)
          (`GameplayStatics.ApplyDamage` (`.HitActor` (`GameplayStatics.BreakHitResult` _outhit)) (`self.AttackDamage`))
          (`self.RandomRoam`))))))

(event `/Game/Blueprints/BPI_Shot.Start Shot`
  (`GameplayStatics.SpawnSoundAttached` "/Game/Audio/SFX/Wolf/Whimpers/SC_Wolf_Death.SC_Wolf_Death" (`self.Audio`) "None" (0.0 0.0 0.0) (struct) "KeepRelativeOffset" false 1.0 1.0 0.0 null null)
  (`self.K2_DestroyActor`))

(fn `UserConstructionScript`)