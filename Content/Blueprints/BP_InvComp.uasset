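; Inventory component that holds a ten-slot item array and shows it through a WB_Inventory widget.
; The inventory input toggles the widget, cursor and input mode.
; Interact line-traces from the camera for a BP_Item, then scans slots in order, stacking on a matching stackable name or filling an empty slot.
; A pickup refreshes the widget and destroys the actor, with IsValid guarding later iterations; no stack limit is enforced.
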(event `self.ReceiveBeginPlay`
  (bind _returnvalue (`|CreateWidget` "/Game/HUD/Inventory/WB_Inventory.WB_Inventory_C"))
  (set `self.Inventory Widget` _returnvalue)
  (`KismetArrayLibrary.Array_Resize` (`self.Items`) 10)
  (`/Game/HUD/Inventory/WB_Inventory.LoadInv` (`self.Inventory Widget`) self))

(event `EnhancedInput|/Game/Blueprints/Input/IA_Inv`
  (params (ActionValue :type Boolean) (ElapsedSeconds :type "Float (double-precision)") (TriggeredSeconds :type "Float (double-precision)") (InputAction :type "InputAction Object Reference" :default "/Game/Blueprints/Input/IA_Inv.IA_Inv"))
  (bind _returnvalue (`GameplayStatics.GetPlayerController` 0))
  (bind _returnvalue_2 (`GameplayStatics.GetPlayerController` 0))
  (bind _inventory_widget (`self.Inventory Widget`))
  (:`Started`
    (if (`Widget.IsVisible` _inventory_widget)
      (`Widget.RemoveFromParent` _inventory_widget)
      (set `PlayerController.bShowMouseCursor` false _returnvalue)
      (`WidgetBlueprintLibrary.SetInputMode_GameOnly` _returnvalue)
      (else
        (set `PlayerController.bShowMouseCursor` true _returnvalue_2)
        (`WidgetBlueprintLibrary.SetInputMode_GameAndUIEx` _returnvalue_2 null)
        (`UserWidget.AddToViewport` _inventory_widget 0)))))

(event `EnhancedInput|/Game/Blueprints/Input/IA_Interact`
  (params (ActionValue :type Boolean) (ElapsedSeconds :type "Float (double-precision)") (TriggeredSeconds :type "Float (double-precision)") (InputAction :type "InputAction Object Reference" :default "/Game/Blueprints/Input/IA_Interact.IA_Interact"))
  (bind _returnvalue (`GameplayStatics.GetPlayerCameraManager` 0))
  (bind _returnvalue_2 (`SceneComponent.K2_GetComponentLocation` (`Actor.RootComponent` _returnvalue)))
  (:`Triggered`
    (bind _asbp_player (cast `/Game/Blueprints/BP_Player` (`GameplayStatics.GetPlayerCharacter` 0)))
    (bind _outhit (`KismetSystemLibrary.LineTraceSingle` _returnvalue_2 (+ _returnvalue_2 (* (`SceneComponent.GetForwardVector` (`Actor.RootComponent` _returnvalue)) (`/Game/Blueprints/BP_Player.InteractDistance` _asbp_player))) "TraceTypeQuery2"))
    (bind _asbp_item (cast `/Game/Blueprints/Inventory/BP_Item` (`.HitActor` (`GameplayStatics.BreakHitResult` _outhit))))
    (for (_array_element _array_index) (`self.Items`)
      (`/Engine/EditorBlueprintResources/StandardMacros.IsValid` _asbp_item
        (:`Is Valid`
          (bind (_name _stackable _quantity) (break `/Game/Blueprints/Inventory/S_ItemStruct` _array_element))
          (bind (_name_2 _stackable_2 _quantity_2) (break `/Game/Blueprints/Inventory/S_ItemStruct` (`/Game/Blueprints/Inventory/BP_Item.Item` _asbp_item)))
          (if (and (`KismetTextLibrary.EqualEqual_TextText` _name _name_2) _stackable_2)
            (bind (_item_name _item_stackable _item_quantity _item_thumbnail _item_mesh) (break `/Game/Blueprints/Inventory/S_ItemStruct` (`/Game/Blueprints/Inventory/BP_Item.Item` _asbp_item)))
            (`KismetArrayLibrary.Array_Set` (`self.Items`) _array_index (make `/Game/Blueprints/Inventory/S_ItemStruct` _item_name _item_stackable (+ _quantity _quantity_2) _item_thumbnail _item_mesh))
            (`/Game/HUD/Inventory/WB_Inventory.LoadInv` (`self.Inventory Widget`) self :!label _label)
            (`Actor.K2_DestroyActor` _asbp_item)
            (elif (== _quantity 0)
              (`KismetArrayLibrary.Array_Set` (`self.Items`) _array_index (`/Game/Blueprints/Inventory/BP_Item.Item` _asbp_item))
              (goto _label))))))))